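; Inventory actor that stores items in a fixed number of slots, each holding an item class and amount, sized on BeginPlay.
; AddItemToInventory looks for a partial stack of stackable items, then an empty slot; non-stackables take one slot each.
; It recurses on overflow and returns any amount that does not fit.
; Helper functions find slots and read item info from class defaults.
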(event EventBeginPlay
  (Utilities|Array|Resize (Variables|Default|GetInventorySlots) (Variables|Default|GetSlotAmount)))

(event Collision|EventActorBeginOverlap
  (params (OtherActor :type Actor%20Object%20Reference)))

(event EventTick
  (params (DeltaSeconds :type Float%20%28single-precision%29)))

(fn ConstructionScript)

(fn IsSlotEmpty
  (params (SlotIndex :type Integer))
  (return (not (Utilities|IsValidClass (.ItemClass (Utilities|Struct|BreakS_InventorySlot (Utilities|Array|Get(acopy) (Variables|Default|GetInventorySlots) SlotIndex)))))))

(fn GetItemInfoatIndex
  (params (ItemIndex :type Integer))
  (bind _inventoryslots (Variables|Default|GetInventorySlots))
  (bind _item (Utilities|Array|Get(acopy) _inventoryslots ItemIndex))
  (bind (_itemclass _itemamount) (Utilities|Struct|BreakS_InventorySlot _item))
  (if (Utilities|IsValidClass _itemclass)
    (return false (Utilities|GetClassDefaults _itemclass) _itemamount)
    (else
      (return true "" 0))))

(fn GetEmptySlotIndex
  (bind _array_index (Utilities|Array|ForEachLoopwithBreak (Variables|Default|GetInventorySlots) :!label _label)
    (:LoopBody
      (if (CallFunction|IsSlotEmpty _array_index)
        (LocalVariables|SetLocal_EmptySlotFound true)
        (LocalVariables|SetLocal_EmptySlotIndex _array_index)
        (goto _label Break)))
    (:Completed
      (return (LocalVariables|GetLocal_EmptySlotFound) (LocalVariables|GetLocal_EmptySlotIndex)))))

(fn GetFreeStackSlotIndex
  (params (ItemClass :type BP%20Master%20Item%20Class%20Reference))
  (bind (_array_element _array_index) (Utilities|Array|ForEachLoopwithBreak (Variables|Default|GetInventorySlots) :!label _label)
    (:LoopBody
      (if (Math|Boolean|ANDBoolean (not (CallFunction|IsSlotEmpty _array_index)) (== (.ItemClass (Utilities|Struct|BreakS_InventorySlot _array_element)) ItemClass) (< (.ItemAmount (Utilities|Struct|BreakS_InventorySlot _array_element)) (Variables|Default|GetMaxStackSize)))
        (LocalVariables|SetLocal_StackFound true)
        (LocalVariables|SetLocal_StackIndex _array_index)
        (goto _label Break)))
    (:Completed
      (return (LocalVariables|GetLocal_StackFound) (LocalVariables|GetLocal_StackIndex)))))

(fn AddItemtoInventory
  (params (ItemClass :type BP%20Master%20Item%20Class%20Reference) (ItemAmount :type Integer))
  (LocalVariables|SetLocal_ItemClass ItemClass)
  (LocalVariables|SetLocal_ItemAmount ItemAmount)
  (if (.CanBeStacked (Utilities|Struct|BreakS_ItemInfo (Utilities|GetClassDefaults ItemClass)))
    (bind (_stackfound _stackslotindex) (CallFunction|GetFreeStackSlotIndex (LocalVariables|GetLocal_ItemClass)))
    (if _stackfound
      (LocalVariables|SetLocal_EmptySlotIndexFound _stackslotindex)
      (if (> (+ (.ItemAmount (Utilities|Struct|BreakS_InventorySlot (Utilities|Array|Get(acopy) (Variables|Default|GetInventorySlots)))) (LocalVariables|GetLocal_ItemAmount)) (Variables|Default|GetMaxStackSize))
        (LocalVariables|SetLocal_ItemAmount (- (+ (.ItemAmount (Utilities|Struct|BreakS_InventorySlot (Utilities|Array|Get(acopy) (Variables|Default|GetInventorySlots)))) (LocalVariables|GetLocal_ItemAmount)) (Variables|Default|GetMaxStackSize)))
        (Utilities|Array|SetArrayElem (Variables|Default|GetInventorySlots) (LocalVariables|GetLocal_EmptySlotIndexFound) (Utilities|Struct|MakeS_InventorySlot (LocalVariables|GetLocal_ItemClass) (Variables|Default|GetMaxStackSize)))
        (bind _itemamountrest (CallFunction|AddItemtoInventory (LocalVariables|GetLocal_ItemClass) (LocalVariables|GetLocal_ItemAmount)))
        (return true _itemamountrest)
        (else
          (Utilities|Array|SetArrayElem (Variables|Default|GetInventorySlots) (LocalVariables|GetLocal_EmptySlotIndexFound) (Utilities|Struct|MakeS_InventorySlot (LocalVariables|GetLocal_ItemClass) (+ (.ItemAmount (Utilities|Struct|BreakS_InventorySlot (Utilities|Array|Get(acopy) (Variables|Default|GetInventorySlots)))) (LocalVariables|GetLocal_ItemAmount))))
          (return true 0)))
      (else
        (bind (_emptyslotfound _emptyslotindex) (CallFunction|GetEmptySlotIndex))
        (if _emptyslotfound
          (bind _output_get (LocalVariables|SetLocal_EmptySlotIndexFound _emptyslotindex))
          (if (> (LocalVariables|GetLocal_ItemAmount) (Variables|Default|GetMaxStackSize))
            (Utilities|Array|SetArrayElem (Variables|Default|GetInventorySlots) _output_get (Utilities|Struct|MakeS_InventorySlot (LocalVariables|GetLocal_ItemClass) 0))
            (bind _itemamountrest_2 (CallFunction|AddItemtoInventory (LocalVariables|GetLocal_ItemClass) (- (LocalVariables|GetLocal_ItemAmount) (Variables|Default|GetMaxStackSize))))
            (return true _itemamountrest_2)
            (else
              (Utilities|Array|SetArrayElem (Variables|Default|GetInventorySlots) (LocalVariables|GetLocal_EmptySlotIndexFound) (Utilities|Struct|MakeS_InventorySlot (LocalVariables|GetLocal_ItemClass) (LocalVariables|GetLocal_ItemAmount)))
              (return true 0)))
          (else
            (return false (LocalVariables|GetLocal_ItemAmount))))))
    (else
      (bind (_emptyslotfound_2 _emptyslotindex_2) (CallFunction|GetEmptySlotIndex))
      (if _emptyslotfound_2
        (bind _output_get_2 (LocalVariables|SetLocal_EmptySlotIndexFound _emptyslotindex_2))
        (Utilities|Array|SetArrayElem (Variables|Default|GetInventorySlots) _output_get_2 (Utilities|Struct|MakeS_InventorySlot (LocalVariables|GetLocal_ItemClass) 1))
        (if (> (LocalVariables|GetLocal_ItemAmount) 1)
          (bind _itemamountrest_3 (CallFunction|AddItemtoInventory (LocalVariables|GetLocal_ItemClass) (- (LocalVariables|GetLocal_ItemAmount) 1)))
          (return true _itemamountrest_3)
          (else
            (return true 0)))
        (else
          (return false (LocalVariables|GetLocal_ItemAmount)))))))

(fn GetItemAmountatIndex
  (params (SlotIndex :type Integer))
  (return (.ItemAmount (Utilities|Struct|BreakS_InventorySlot (Utilities|Array|Get(acopy) (Variables|Default|GetInventorySlots))))))