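; BP_ItemPickup is a world pickup that gives an item class and amount to the player's inventory.
; When a ThirdPersonCharacter overlaps its sphere, it calls AddItemToInventory on that character's inventory reference.
; After a successful add, it keeps any leftover amount, or destroys itself if none remains.
; The construction script fills its name and amount text from the item's class defaults and ItemAmount; pickup does not refresh them.
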(event OnComponentBeginOverlap(Sphere)
  (params (OverlappedComponent :type Primitive%20Component%20Object%20Reference) (OtherActor :type Actor%20Object%20Reference) (OtherComp :type Primitive%20Component%20Object%20Reference) (OtherBodyIndex :type Integer) (bFromSweep :type Boolean) (SweepResult :type Hit%20Result%20Structure%20%28by%20ref%29))
  (bind _asthird_person_character (Utilities|Casting|CastToThirdPersonCharacter OtherActor))
  (Utilities|IsValid (Variables|/Game/ThirdPersonBP/Blueprints/ThirdPersonCharacter.ThirdPersonCharacter_C|GetInventoryReference _asthird_person_character)
    (:Is%20Valid
      (bind (_itemadded _itemamountrest) (Default|AddItemtoInventory (Variables|/Game/ThirdPersonBP/Blueprints/ThirdPersonCharacter.ThirdPersonCharacter_C|GetInventoryReference _asthird_person_character) (Variables|Default|GetItemClass) (Variables|Default|GetItemAmount)))
      (if _itemadded
        (if (> _itemamountrest 0)
          (Variables|Default|SetItemAmount _itemamountrest)
          (else
            (Actor|DestroyActor)))))))

(event EventBeginPlay)

(event Collision|EventActorBeginOverlap
  (params (OtherActor :type Actor%20Object%20Reference)))

(event EventTick
  (params (DeltaSeconds :type Float%20%28single-precision%29)))

(fn ConstructionScript
  (Rendering|Components|TextRender|SetText (Variables|Default|GetItemNameText) (.Name (Utilities|Struct|BreakS_ItemInfo (Utilities|GetClassDefaults (Variables|Default|GetItemClass)))))
  (Rendering|Components|TextRender|SetText (Variables|Default|GetItemAmountText) (Utilities|Text|ToText(Integer) (Variables|Default|GetItemAmount))))